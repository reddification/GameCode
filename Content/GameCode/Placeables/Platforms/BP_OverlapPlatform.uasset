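; BP_OverlapPlatform is a placeable platform that activates while something overlaps its trigger box.
; Beginning an overlap calls Start and ending one calls ReverseStop, with no actor filtering or overlap counting in this graph.
; The construction script sizes the box from the platform mesh's local bounds times PlatformCollisionScale, using full size as extent, and raises it by the mesh's height.
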(event OnComponentBeginOverlap(Box)
  (params (OverlappedComponent :type Primitive%20Component%20Object%20Reference) (OtherActor :type Actor%20Object%20Reference) (OtherComp :type Primitive%20Component%20Object%20Reference) (OtherBodyIndex :type Integer) (bFromSweep :type Boolean) (SweepResult :type Hit%20Result%20Structure%20%28by%20ref%29))
  (Class|BasePlatform|Start))

(event OnComponentEndOverlap(Box)
  (params (OverlappedComponent :type Primitive%20Component%20Object%20Reference) (OtherActor :type Actor%20Object%20Reference) (OtherComp :type Primitive%20Component%20Object%20Reference) (OtherBodyIndex :type Integer))
  (Class|BasePlatform|ReverseStop))

(fn ConstructionScript
  (bind _box (Variables|Default|GetBox))
  (bind _platformmesh (Variables|Default|GetPlatformMesh))
  (bind _platformcollisionscale (LocalVariables|GetPlatformCollisionScale))
  (bind (_min _max) (Components|StaticMesh|GetLocalBounds _platformmesh))
  (bind _returnvalue (- _max _min))
  (bind (_x _y _z) (Math|Vector|BreakVector _returnvalue))
  (Components|Box|SetBoxExtent _box (Math|Vector|MakeVector (* _platformcollisionscale _x) (* _platformcollisionscale _y) (* _platformcollisionscale _z)) true)
  (Transformation|SetRelativeLocation _box (Math|Vector|MakeVector 0.0 0.0 _z) false false))